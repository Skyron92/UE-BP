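; BP_Interuptor is a pressure-plate style switch that signals linked doors when the third-person character stands on it.
; Box overlap begin and end set PlayerIsOverlap true or false on every door in the BPDoor array.
; The Interruptor component sinks on entry and rises on exit; the offset runs inside the loop, so travel scales with the number of linked doors.
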(event `self.Box.OnComponentBeginOverlap`
  (params (OverlappedComponent :type "PrimitiveComponent Object Reference") (OtherActor :type "Actor Object Reference") (OtherComp :type "PrimitiveComponent Object Reference") (OtherBodyIndex :type Integer) (bFromSweep :type Boolean) (SweepResult :type "HitResult Structure (by ref)"))
  (cast `/Game/ThirdPerson/Blueprints/BP_ThirdPersonCharacter` OtherActor)
  (for _array_element (`self.BP Door`)
    (set `/Game/BluePrints/BP_Door.playerIsOverlap` true _array_element)
    (`SceneComponent.K2_AddLocalOffset` (`self.Interruptor`) (0.0 0.0 -1.0) false false)))

(event `self.Box.OnComponentEndOverlap`
  (params (OverlappedComponent :type "PrimitiveComponent Object Reference") (OtherActor :type "Actor Object Reference") (OtherComp :type "PrimitiveComponent Object Reference") (OtherBodyIndex :type Integer))
  (cast `/Game/ThirdPerson/Blueprints/BP_ThirdPersonCharacter` OtherActor)
  (for _array_element (`self.BP Door`)
    (set `/Game/BluePrints/BP_Door.playerIsOverlap` false _array_element)
    (`SceneComponent.K2_AddLocalOffset` (`self.Interruptor`) (0.0 0.0 1.0) false false)))

(fn `UserConstructionScript`)