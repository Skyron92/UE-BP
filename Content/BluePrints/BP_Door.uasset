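; BP_Door is an automatic sliding door that opens while the third-person player character stands in its trigger box and closes when the character leaves.
; Box overlap events cast the other actor to BP_ThirdPersonCharacter and set the PlayerIsOverlap flag.
; Each Tick reads that flag and nudges the Door component along local X between its limits by a fixed per-frame step, so slide speed depends on frame rate.
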(event `self.ReceiveTick`
  (params (DeltaSeconds :type "Float (single-precision)"))
  (bind _door (`self.Door`))
  (bind _x (.x (.location (`SceneComponent.GetRelativeTransform` _door))))
  (if (and (>= _x -100.0) (stale `self.Box.OnComponentBeginOverlap` _output_get))
    (`SceneComponent.K2_AddLocalOffset` _door (-2.0 0.0 0.0) false false)
    (elif (and (<= _x 0.0) (not (stale `self.Box.OnComponentEndOverlap` _output_get)))
      (`SceneComponent.K2_AddLocalOffset` _door (2.0 0.0 0.0) false false))))

(event `self.Box.OnComponentBeginOverlap`
  (params (OverlappedComponent :type "PrimitiveComponent Object Reference") (OtherActor :type "Actor Object Reference") (OtherComp :type "PrimitiveComponent Object Reference") (OtherBodyIndex :type Integer) (bFromSweep :type Boolean) (SweepResult :type "HitResult Structure (by ref)"))
  (cast `/Game/ThirdPerson/Blueprints/BP_ThirdPersonCharacter` OtherActor)
  (bind _output_get (set `self.playerIsOverlap` true)))

(event `self.Box.OnComponentEndOverlap`
  (params (OverlappedComponent :type "PrimitiveComponent Object Reference") (OtherActor :type "Actor Object Reference") (OtherComp :type "PrimitiveComponent Object Reference") (OtherBodyIndex :type Integer))
  (cast `/Game/ThirdPerson/Blueprints/BP_ThirdPersonCharacter` OtherActor)
  (bind _output_get (set `self.playerIsOverlap` false)))

(fn `UserConstructionScript`)