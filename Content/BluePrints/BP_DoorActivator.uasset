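; BP_DoorActivator is a pressure switch that sinks while the third-person character stands in its trigger box and rises on exit.
; It starts responding only after a one-shot EventLauncher event calls SetActive, which turns the switch green through a dynamic material and enables particles.
; Once active, each step onto it sends ActivateMessage to every entry in BPControlables implementing BPI_InteruptorControlable.
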(event `self.ReceiveBeginPlay`
  ;[1 0.5521 0.5521] Event Listenner
  (add `/Game/BluePrints/BP_InteruptorEventLauncher.ActivateControlables` (`self.Event Launcher`) (delegate `OnActivate`)))

(event `OnActivate`
  ;[1 0.5521 0.5521] Event Listenner
  (`self.SetActive`)
  (remove `/Game/BluePrints/BP_InteruptorEventLauncher.ActivateControlables` (`self.Event Launcher`) (delegate `OnActivate`)))

(event `self.Box.OnComponentBeginOverlap`
  (params (OverlappedComponent :type "PrimitiveComponent Object Reference") (OtherActor :type "Actor Object Reference") (OtherComp :type "PrimitiveComponent Object Reference") (OtherBodyIndex :type Integer) (bFromSweep :type Boolean) (SweepResult :type "HitResult Structure (by ref)"))
  (cast `/Game/ThirdPerson/Blueprints/BP_ThirdPersonCharacter` OtherActor)
  ;[0.598 1 0.6062] Interruptor animation
  (`SceneComponent.K2_AddLocalOffset` (`self.Interruptor`) (0.0 0.0 -4.0) false false)
  ;[1 0.6198 0.6798] Activate InteruptorControlables
  (if (`self.IsActive`)
    (for _array_element (`self.BP controlables`)
      (if (`KismetSystemLibrary.DoesImplementInterface` _array_element "/Game/BluePrints/BPI_InteruptorControlable.BPI_InteruptorControlable_C")
        (message `/Game/BluePrints/BPI_InteruptorControlable.Activate` _array_element)))))

(event `self.Box.OnComponentEndOverlap`
  (params (OverlappedComponent :type "PrimitiveComponent Object Reference") (OtherActor :type "Actor Object Reference") (OtherComp :type "PrimitiveComponent Object Reference") (OtherBodyIndex :type Integer))
  (cast `/Game/ThirdPerson/Blueprints/BP_ThirdPersonCharacter` OtherActor)
  ;[0.631 1 0.6133] Interruptor animation
  (`SceneComponent.K2_AddLocalOffset` (`self.Interruptor`) (0.0 0.0 4.0) false false))

(fn `SetActive`
  (set `self.IsActive` true)
  (bind _returnvalue (`PrimitiveComponent.CreateDynamicMaterialInstance` (`self.Interruptor`) 0 null "None"))
  (`MaterialInstanceDynamic.SetVectorParameterValue` _returnvalue "Colour" (struct :`G` 1.0 :`B` 0.121026 :`A` 1.0))
  (bind _output_get (set `self.Particles` (`self.Particles`)))
  (`ActorComponent.SetActive` _output_get true false))

(fn `UserConstructionScript`)