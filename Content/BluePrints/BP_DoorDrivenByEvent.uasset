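; Sliding door Blueprint that opens and closes in response to an external event launcher rather than its own overlap detection.
; On BeginPlay it binds to EventLauncher, and each activation flips the PlayerIsOverlap flag, which acts as the open/closed state despite its name.
; Tick nudges the Door component along local X by a fixed per-frame step between closed and open limits, so speed depends on frame rate.
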(event `self.ReceiveBeginPlay`
  (add `/Game/BluePrints/BP_InteruptorEventLauncher.ActivateControlables` (`self.Event launcher`) (delegate `OnActivate`)))

(event `OnActivate`
  (`self.ToggleDoor`))

(event `self.ReceiveTick`
  (params (DeltaSeconds :type "Float (single-precision)"))
  (bind _playerisoverlap (`self.playerIsOverlap`))
  (bind _door (`self.Door`))
  (bind _x (.x (.location (`SceneComponent.GetRelativeTransform` _door))))
  (if (and (>= _x -100.0) _playerisoverlap)
    (`SceneComponent.K2_AddLocalOffset` _door (-2.0 0.0 0.0) false false)
    (elif (and (<= _x 0.0) (not _playerisoverlap))
      (`SceneComponent.K2_AddLocalOffset` _door (2.0 0.0 0.0) false false))))

(fn `ToggleDoor`
  (set `self.playerIsOverlap` (not (`self.playerIsOverlap`))))

(fn `UserConstructionScript`)